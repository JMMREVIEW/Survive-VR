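; Fixed-camera volume that blends the view to a cine camera sliding along a spline as the player moves through it.
; Overlap enables Tick, which maps player progress on PlayerSpline onto CameraSpline, optionally reversed, with optional focus tracking.
; Soft Lock mode follows the player or spline rotation, slowing and holding yaw at limits; Look At tracks yaw with fixed pitch.
; Construction script applies lens settings and previews both spline positions.
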(event `self.ReceiveBeginPlay`
  (`SceneComponent.SetHiddenInGame` (`self.PlayerReference`) true true)
  (`KismetSystemLibrary.K2_SetTimerDelegate` (delegate `CheckForPlayer`) 0.1))

(event `CheckForPlayer`
  (if (`PrimitiveComponent.IsOverlappingActor` (`self.Collision`) (`GameplayStatics.GetPlayerCharacter` 0))
    (`self.OnFixedCameraOverlap`)))

(event `self.Collision.OnComponentBeginOverlap`
  (params (OverlappedComponent :type "PrimitiveComponent Object Reference") (OtherActor :type "Actor Object Reference") (OtherComp :type "PrimitiveComponent Object Reference") (OtherBodyIndex :type Integer) (bFromSweep :type Boolean) (SweepResult :type "HitResult Structure (by ref)"))
  (if (== OtherActor (`GameplayStatics.GetPlayerCharacter` 0))
    (`self.OnFixedCameraOverlap`)))

(event `self.Collision.OnComponentEndOverlap`
  (params (OverlappedComponent :type "PrimitiveComponent Object Reference") (OtherActor :type "Actor Object Reference") (OtherComp :type "PrimitiveComponent Object Reference") (OtherBodyIndex :type Integer))
  (if (== OtherActor (`GameplayStatics.GetPlayerCharacter` 0))
    (`self.OnFixedCameraEndOverlap`)))

(event `self.ReceiveTick`
  (params (DeltaSeconds :type "Float (single-precision)"))
  (bind _returnvalue (`GameplayStatics.GetPlayerPawn` 0))
  (bind _returnvalue_2 (`SplineComponent.GetSplineLength` (`self.CameraSpline`)))
  (bind (_returnvalue_roll _returnvalue_pitch _returnvalue_yaw) (`KismetMathLibrary.BreakRotator` (`SceneComponent.K2_GetComponentRotation` (`self.CineCamera`))))
  (bind (_returnvalue_roll_2 _returnvalue_pitch_2 _returnvalue_yaw_2) (`KismetMathLibrary.BreakRotator` (`SplineComponent.GetRotationAtDistanceAlongSpline` (`self.CameraSpline`) (`self.CameraDistanceAlongSpline`) "World")))
  (bind (_returnvalue_location _returnvalue_rotation) (`KismetMathLibrary.BreakTransform` (`SplineComponent.GetTransformAtDistanceAlongSpline` (`self.PlayerSpline`) (`self.PlayerDistanceAlongSpline`) "World" false)))
  (bind _returnvalue_3 (`self.K2_GetActorLocation` (`GameplayStatics.GetPlayerPawn` 0)))
  (bind (_returnvalue_roll_3 _returnvalue_pitch_3 _returnvalue_yaw_3) (`KismetMathLibrary.BreakRotator` (`KismetMathLibrary.FindLookAtRotation` (`SceneComponent.K2_GetComponentLocation` (`self.CineCamera`)) (`self.K2_GetActorLocation` (`GameplayStatics.GetPlayerPawn` 0)))))
  (bind _returnvalue_4 (`KismetMathLibrary.GetRightVector` _returnvalue_rotation))
  ; Logic to get player position along spline
  (set `self.Delta Seconds` DeltaSeconds)
  (bind _output_get (set `self.PlayerDistanceAlongSpline` (`SplineComponent.GetDistanceAlongSplineAtSplineInputKey` (`self.PlayerSpline`) (`SplineComponent.FindInputKeyClosestToWorldLocation` (`self.PlayerSpline`) (+ (`self.K2_GetActorLocation` _returnvalue) (`self.GetActorForwardVector` _returnvalue))))))
  (bind _returnvalue_5 (`KismetMathLibrary.Lerp` (select `bool` (`self.CameraReverse`) :`true` _returnvalue_2 :!type "Float (double-precision)") (select `bool` (`self.CameraReverse`) :`false` _returnvalue_2 :!type "Float (double-precision)") (`KismetMathLibrary.MapRangeClamped` _output_get 0.0 (`SplineComponent.GetSplineLength` (`self.PlayerSpline`)) 0.0 1.0)))
  (set `self.CameraDistanceAlongSpline` _returnvalue_5)
  (bind _returnvalue_6 (`SplineComponent.GetLocationAtDistanceAlongSpline` (`self.CameraSpline`) _returnvalue_5 "World"))
  (`SceneComponent.K2_SetWorldLocation` (`self.CineCamera`) _returnvalue_6 false false)
  (switch `/Game/Blueprints/FixedCamera/ECameraMode` (`self.ECameraMode`)
    (:`NewEnumerator1`
      (if (or (`self.VerticalPlayerFollow`) (`self.HorizontalPlayerFollow`))
        ; If HorizontalPlayerFollow true AND Camsoftlock isn't 0 then set soft lock and check to see if look at rotation is outside of soft lock
        (if (and (`self.HorizontalPlayerFollow`) (!= (`self.CameraSoftLockValue`) 0.0))
          (`self.SetSoftLock` _returnvalue_yaw_3))
        (`SceneComponent.K2_SetWorldRotation` (`self.CineCamera`) (`KismetMathLibrary.RInterpTo` (`SceneComponent.K2_GetComponentRotation` (`self.CineCamera`)) (`KismetMathLibrary.MakeRotator` _returnvalue_roll_2 (select `bool` (`self.VerticalPlayerFollow`) :`false` _returnvalue_pitch_2 :`true` _returnvalue_pitch_3) (select `bool` (`self.HorizontalPlayerFollow`) :`false` _returnvalue_yaw_2 :`true` (select `bool` (`self.IsOutsideSoftLock`) :`false` _returnvalue_yaw_3 :`true` _returnvalue_yaw))) (`self.Delta Seconds`) (`self.Interp Speed`)) false false)
        (else
          (`SceneComponent.K2_SetWorldRotation` (`self.CineCamera`) (`SplineComponent.GetRotationAtDistanceAlongSpline` (`self.CameraSpline`) (`self.CameraDistanceAlongSpline`) "World") false false))))
    (:`NewEnumerator2`
      (`SceneComponent.K2_SetWorldRotation` (`self.CineCamera`) (`KismetMathLibrary.MakeRotator` 0.0 (`self.PerCameraPitchOffset`) (.yaw (`KismetMathLibrary.FindLookAtRotation` (+ _returnvalue_6 (`KismetMathLibrary.VInterpTo` (0.0 0.0 0.0) (* (* (`KismetMathLibrary.Dot_VectorVector` (- _returnvalue_3 (`SplineComponent.FindLocationClosestToWorldLocation` (`self.PlayerSpline`) _returnvalue_3 "World")) _returnvalue_4) (`self.OffsetScale`)) _returnvalue_4))) (`self.K2_GetActorLocation` (`GameplayStatics.GetPlayerPawn` 0))))) false false))))

(fn `OnFixedCameraEndOverlap`
  (`self.SetActorTickEnabled` false))

(fn `OnFixedCameraOverlap`
  (`self.SetActorTickEnabled` true)
  (`PlayerController.SetViewTargetWithBlend` (`GameplayStatics.GetPlayerController` 0) self (`self.Blend Time`) "VTBlend_Linear" 0.0 false)
  (if (`self.ShouldFocusOnPlayer`)
    (set `CineCameraComponent.FocusSettings` (make `CameraFocusSettings` "Tracking" 100000.0 (make `CameraTrackingFocusSettings` (`|ConvertAsset` (`GameplayStatics.GetPlayerCharacter` 0)))) (`self.CineCamera`))))

(fn `SetCameraSettings`
  (set `CineCameraComponent.CurrentAperture` (`self.Camera Aperture`) (`self.CineCamera`))
  (set `CineCameraComponent.CurrentFocalLength` (`self.CameraFocalLenght`) (`self.CineCamera`)))

(fn `SetSoftLock`
  (params (CameraRotation :type "Float (double-precision)"))
  (bind _camerasoftlockvalue (`self.CameraSoftLockValue`))
  (bind (_returnvalue_roll _returnvalue_pitch _returnvalue_yaw) (`KismetMathLibrary.BreakRotator` (`SplineComponent.GetRotationAtDistanceAlongSpline` (`self.CameraSpline`) (`self.CameraDistanceAlongSpline`) "World")))
  (bind _returnvalue (- _returnvalue_yaw _camerasoftlockvalue))
  (bind _returnvalue_2 (+ _returnvalue_yaw _camerasoftlockvalue))
  (set `self.IsOutsideSoftLock` (not (`KismetMathLibrary.InRange_FloatFloat` (`local.CameraRotation`) _returnvalue _returnvalue_2)))
  (set `self.Interp Speed` (`KismetMathLibrary.MapRangeClamped` (`local.CameraRotation`) _returnvalue_yaw (select `bool` (> (`local.CameraRotation`) _returnvalue_yaw) :`false` _returnvalue :`true` _returnvalue_2) (`self.SoftLockSpeedMax`) (`self.SoftLockSpeedMin`)))
  (return))

(fn `SnapToSpline`
  (bind _returnvalue (`SplineComponent.GetSplineLength` (`self.CameraSpline`)))
  (bind _returnvalue_2 (`KismetMathLibrary.Lerp` (select `bool` (`self.CameraReverse`) :`true` _returnvalue :!type "Float (double-precision)") (select `bool` (`self.CameraReverse`) :`false` _returnvalue :!type "Float (double-precision)") (`self.EditorCameraPoint`)))
  (`SceneComponent.K2_SetWorldTransform` (`self.CineCamera`) (`KismetMathLibrary.MakeTransform` (`SplineComponent.GetLocationAtDistanceAlongSpline` (`self.CameraSpline`) _returnvalue_2 "World") (`SplineComponent.GetRotationAtDistanceAlongSpline` (`self.CameraSpline`) _returnvalue_2 "World")) false false)
  (`SceneComponent.K2_SetWorldLocation` (`self.PlayerReference`) (`SplineComponent.GetLocationAtDistanceAlongSpline` (`self.PlayerSpline`) (`KismetMathLibrary.Lerp` 0.0 (`SplineComponent.GetSplineLength` (`self.PlayerSpline`)) (`self.EditorCameraPoint`)) "World") false false))

(fn `UserConstructionScript`
  (`self.SetCameraSettings`)
  (`self.SnapToSpline`))